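; Base enemy Blueprint, using a zombie attack montage, that chases a player pawn, melee attacks it and takes damage.
; ChasePlayer runs AI MoveTo, then fires a DoOnce-gated Attack on arrival if still alive.
; Attack halts movement during the montage; its notify sphere-overlaps pawns, sending damage, and only a hit restarts the chase and resets the gate.
; ApplyDmg updates health and death state, disabling mesh collision when dead.
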(event `self.ReceiveBeginPlay`
  (`KismetArrayLibrary.Array_Add` (`self.Actors to Ignore`) self))

(event `/Game/BP/Interface/BPI_Damageable.ApplyDmg`
  (params (Damage :type "Float (single-precision)"))
  (bind _mesh (`self.Mesh`))
  (`self.CalculateHealth` (* Damage -1.0))
  (`self.CalculateDead`)
  (if (`self.isDead`)
    (`PrimitiveComponent.SetCollisionObjectType` _mesh "ECC_WorldStatic")
    (`PrimitiveComponent.SetCollisionEnabled` _mesh "NoCollision")))

(event `ChasePlayer`
  (params (Pawn :type "Pawn Object Reference"))
  (bind _output_get (set `self.Player` Pawn))
  (`|AIMoveTo` self (0.0 0.0 0.0) _output_get
    (:`OnSuccess`
      (if (not (`self.isDead`))
        (`/Engine/EditorBlueprintResources/StandardMacros.DoOnce` false :!label _label
          (:`Completed`
            (`self.Attack`)))))))

(event `Attack`
  (bind _charactermovement (`self.CharacterMovement`))
  (`CharacterMovementComponent.DisableMovement` _charactermovement)
  (`|PlayMontage` (`self.Mesh`) "/Game/Enemy/Enemy1/Animations/Zombie_Attack_Montage.Zombie_Attack_Montage"
    (:`OnCompleted`
      (`CharacterMovementComponent.SetMovementMode` _charactermovement "MOVE_Walking" 0))
    (:`OnNotifyBegin`
      (bind _outactors (`KismetSystemLibrary.SphereOverlapActors` (`SceneComponent.K2_GetComponentLocation` (`self.SphereAttack`)) 0.0 (`|MakeArray` "ObjectTypeQuery3" :!type "EObjectTypeQuery Enum") null (`self.Actors to Ignore`)))
      (for _array_element _outactors
        (message `/Game/BP/Interface/BPI_Damageable.ApplyDmg` _array_element (`self.Damage`))
        (`self.ChasePlayer` (`self.Player`))
        (goto _label :!via `Reset`)))))

(fn `UserConstructionScript`)