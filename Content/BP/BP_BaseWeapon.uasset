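; Base weapon Blueprint that the player picks up on overlap and that damages non-player actors it hits.
; Overlapping the sphere sends an equip interface message to the player with the weapon and katana socket name, then stops mesh physics simulation.
; The hit capsule sends damage messages to overlapped actors not tagged Player.
; Interface events toggle the capsule's collision and visibility together, starting disabled at BeginPlay.
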(event `self.ReceiveBeginPlay`
  (`self.DisableCollision`))

(event `self.Sphere.OnComponentBeginOverlap`
  (params (OverlappedComponent :type "PrimitiveComponent Object Reference") (OtherActor :type "Actor Object Reference") (OtherComp :type "PrimitiveComponent Object Reference") (OtherBodyIndex :type Integer) (bFromSweep :type Boolean) (SweepResult :type "HitResult Structure (by ref)"))
  (if (`self.ActorHasTag` OtherActor "Player")
    (message `/Game/BP/Interface/BPI_Player.EquipWeapon` OtherActor self (`self.CatanaAttachSocketName`))
    (`PrimitiveComponent.SetSimulatePhysics` (`self.Mesh`) false)))

(event `self.HitCapsuleCollision.OnComponentBeginOverlap`
  (params (OverlappedComponent :type "PrimitiveComponent Object Reference") (OtherActor :type "Actor Object Reference") (OtherComp :type "PrimitiveComponent Object Reference") (OtherBodyIndex :type Integer) (bFromSweep :type Boolean) (SweepResult :type "HitResult Structure (by ref)"))
  (if (not (`self.ActorHasTag` OtherActor "Player"))
    (message `/Game/BP/Interface/BPI_Damageable.ApplyDmg` OtherActor (`self.Damage`))))

(event `self.EnableCollision`
  (bind _hitcapsulecollision (`self.HitCapsuleCollision`))
  ;[0.6531 0.7609 1] BPI
  (`PrimitiveComponent.SetCollisionEnabled` _hitcapsulecollision "QueryAndPhysics")
  (`SceneComponent.SetHiddenInGame` _hitcapsulecollision false true))

(event `self.DisableCollision`
  (bind _hitcapsulecollision (`self.HitCapsuleCollision`))
  ;[0.6531 0.7609 1] BPI
  (`PrimitiveComponent.SetCollisionEnabled` _hitcapsulecollision "NoCollision")
  (`SceneComponent.SetHiddenInGame` _hitcapsulecollision true true))

(fn `UserConstructionScript`)